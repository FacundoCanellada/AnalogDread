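; Rotating picture frame puzzle piece, where all placed frames must reach their answer position to complete the puzzle.
; Interaction plays a sound and turns the frame 90 degrees by timeline through four positions, ignoring rotation while moving.
; It sets Finalized by comparing the next position to the answer, before rotation starts.
; Each instance polls all frames on a looping timer, then stops and fires the puzzle-completed dispatcher.
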(event Custom|RotatePicture
  ;[0.15 0 0.1301] Rotate picture system
  (if (not (Variables|Default|GetFrameMoving))
    (Variables|Default|SetFrameMoving true)
    (Audio|PlaySound2D "/Game/Facu/Sounds/SlidePicture.SlidePicture" 1.0 1.0 0.0 0 0)
    (bind _alpha (Timeline|PaintingRotation_TL PlayFromStart)
      (:Update
        (Transformation|SetRelativeRotation (Variables|Default|GetFrame) (Math|Rotator|MakeRotator 0.0 (Math|Float|Lerp (.pitch (Variables|Default|GetStartingRotationFrame)) (- (.pitch (Variables|Default|GetStartingRotationFrame)) 9e+01) _alpha) 0.0) false false))
      (:Finished
        (Variables|Default|SetStartingRotationFrame (Math|Rotator|MakeRotator 0.0 (Math|Float|Lerp (.pitch (Variables|Default|GetStartingRotationFrame)) (- (.pitch (Variables|Default|GetStartingRotationFrame)) 9e+01) _alpha) 0.0))
        (Variables|Default|SetFrameMoving false)
        (bind _result (Math|Integer|IncrementInt (Variables|Default|GetFramePosition))
          (:%20%20
            (bind _output_get (Variables|Default|SetFramePosition _result))
            (if (> _output_get 3)
              (Variables|Default|SetFramePosition 0))))))))

(event Custom|CheckPuzzle
  ;[0.15 0 0.1301] Check Puzzle
  (Variables|Default|SetPuzzleSolved true)
  (for _array_element (Variables|Default|GetAllPicturesFrames)
    (if (not (Variables|BP_PictureFrameMaster_Puzzle_C|GetFinalized _array_element))
      (Variables|Default|SetPuzzleSolved false)))
  (if (Variables|Default|GetPuzzleSolved)
    (Utilities|Time|ClearandInvalidateTimerbyHandle (stale EventBeginPlay _returnvalue))
    (Default|CallEVDPuzzleCompleted)))

(event EventBeginPlay
  ;[0.15 0 0.1301] Check Puzzle
  (Variables|Default|SetStartingRotationFrame (Variables|/Script/Engine.SceneComponent|GetRelativeRotation (Variables|Default|GetFrame)))
  (bind _outactors (Actor|GetAllActorsOfClass "BP_PictureFrameMaster_Puzzle_C"))
  (Variables|Default|SetAllPicturesFrames _outactors)
  (bind _returnvalue (Utilities|Time|SetTimerbyEvent (delegate Custom|CheckPuzzle) 0.25 true)))

(event EventInteraction
  ;[0.15 0 0.1301] Interaction System
  (if (== (+ (Variables|Default|GetFramePosition) 1) (Variables|Default|GetPuzzleAnsewer))
    (Variables|Default|SetFinalized true)
    (CallFunction|RotatePicture)
    (else
      (Variables|Default|SetFinalized false)
      (CallFunction|RotatePicture))))

(fn ConstructionScript
  (|CallParentFunction))