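; BPC_DialogueComponent is a dialogue component that steps through an array of lines and shows them in a WB_Dialogue widget.
; On BeginPlay it creates the widget with its name color and opacity settings.
; Each Speech call pauses the game, sends the current line, speaker name and text delay to the widget, then advances the index.
; Once the index passes the last line, it resets, clears the widget and unpauses.
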(event Custom|Speech
  (bind _dialogue (Variables|Default|GetDialogue))
  (Game|SetGamePaused true)
  (Default|IncomingText (Variables|Default|GetWB_DialogueRef) (Utilities|Array|Get(acopy) _dialogue (Variables|Default|GetCurrentDialogue)) (Variables|Default|GetDelayText) (Variables|Default|GetName))
  (bind _result (Math|Integer|IncrementInt (Variables|Default|GetCurrentDialogue))
    (:%20%20
      (if (>= _result (+ (Utilities|Array|Length _dialogue) 1))
        (Variables|Default|SetCurrentDialogue 0)
        (Default|ClearScreen (Variables|Default|GetWB_DialogueRef))
        (Game|SetGamePaused false)))))

(event EventBeginPlay
  (bind _returnvalue (UserInterface|CreateWidget "/Game/Facu/Widgets/WB_Dialogue.WB_Dialogue_C" 0 (Variables|Default|GetName%20Color) (Variables|Default|GetDialogue%20Opacity)))
  (Variables|Default|SetWB_DialogueRef _returnvalue))