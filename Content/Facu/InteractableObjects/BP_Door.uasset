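; Interactable hinged door that swings away from the player, with optional key lock and auto-close.
; Interaction toggles the door through a reversible timeline, using a dot product to pick swing direction, with handle animation and sounds.
; When locked, it compares DoorKeyID to only the last key in the player's Keys, then unlocks and opens or shakes.
; A looping timer closes it once the player exceeds CloseDistance.
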(event Custom|OpenCloseDoor
  (bind _self self)
  ;[0 0.06301 0.15] Open/Close logic
  (CallFunction|Sounds)
  (if (Variables|Default|GetDoorClosed?)
    (Variables|Default|SetDoorClosed? false)
    (CallFunction|RotateDoorHandle)
    (Variables|Default|SetDotProduct (Math|Vector|DotProduct (Math|Vector|Normalize (- (Transformation|GetActorLocation _self) (Transformation|GetActorLocation (Variables|Default|GetPlayer%20Ref)))) (Transformation|GetActorRightVector _self)))
    (bind _alpha (Timeline|Door_TL PlayFromStart)
      (:Update
        (Transformation|SetRelativeRotation (Variables|Default|GetDoor) (Math|Rotator|MakeRotator 0.0 0.0 (Math|Float|Lerp 0.0 (Math|Float|SelectFloat 85.0 -85.0 (>= (Variables|Default|GetDotProduct) 0.0)) _alpha)) false false)))
    (else
      (Variables|Default|SetDoorClosed? true)
      (Timeline|Door_TL Reverse))))

(event Custom|AutoClose
  ;[0 0.06301 0.15] Auto/Close Door
  (if (Variables|Default|GetAutoClose?)
    (Utilities|Time|SetTimerbyEvent (delegate Custom|Door%20AutoClose) 2.0 true)))

(event Custom|Door%20AutoClose
  ;[0 0.06301 0.15] Auto/Close Door
  (if (not (Variables|Default|GetDoorClosed?))
    (if (> (Math|Vector|Distance(Vector) (Transformation|GetActorLocation (Variables|Default|GetPlayer%20Ref)) (Transformation|GetActorLocation)) (Variables|Default|GetCloseDistance))
      (CallFunction|OpenCloseDoor))))

(event Custom|CheckForKey
  ;[0 0.06301 0.15] CheckKey
  (for _array_element (Variables|/Game/Facu/Blueprints/Character/BP_FirstPersonFacu.BP_FirstPersonFacu_C|GetKeys (Variables|Default|GetPlayer%20Ref))
    _)
  (if (Utilities|Enum|Equal(Enum) _array_element (Variables|Default|GetDoorKeyID))
    (CallFunction|UnlockDoor)
    (else
      (CallFunction|ShakeDoor))))

(event Custom|RotateDoorHandle
  ;[0 0.06301 0.15 1] RotateHandle
  (bind _alpha (Timeline|RotateHandle_TL PlayFromStart)
    (:Update
      (Transformation|SetRelativeRotation (Variables|Default|GetDoorHandle1) (Math|Rotator|MakeRotator _alpha 0.0 0.0) false false))))

(event Custom|UnlockDoor
  (bind _unlockdoorsound (Variables|Default|GetUnlockDoorSound))
  ;[0 0.06301 0.15] Unlock door logic
  (Variables|Default|SetLocked? false)
  (Audio|PlaySoundatLocation _unlockdoorsound (Transformation|GetWorldLocation (Variables|Default|GetDoor)) "0, 0, 0" 1.0 1.0 0.0 0 0 0 0)
  (Utilities|FlowControl|Delay (Variables|/Script/Engine.SoundBase|GetDuration _unlockdoorsound))
  (CallFunction|OpenCloseDoor))

(event Custom|ShakeDoor
  ;[0 0.06301 0.15] ShakeDoor
  (CallFunction|RotateDoorHandle)
  (Audio|PlaySoundatLocation (Variables|Default|GetLockDoorSound) (Transformation|GetWorldLocation (Variables|Default|GetDoor)) "0, 0, 0" 1.0 1.0 0.0 0 0 0 0)
  (bind _alpha (Timeline|ShakeDoor_TL PlayFromStart)
    (:Update
      (Transformation|SetRelativeRotation (Variables|Default|GetDoor) (Math|Rotator|MakeRotator 0.0 0.0 _alpha) false false))))

(event Collision|EventActorBeginOverlap
  (params (OtherActor :type Actor%20Object%20Reference)))

(event EventTick
  (params (DeltaSeconds :type Float%20%28single-precision%29)))

(event EventBeginPlay
  (bind _asbp_first_person_facu (Utilities|Casting|CastToBP_FirstPersonFacu (Game|GetPlayerCharacter 0)))
  (Variables|Default|SetPlayer%20Ref _asbp_first_person_facu)
  (CallFunction|AutoClose))

(event EventInteraction
  ;[0 0.06301 0.15] Interaction System
  (if (Variables|Default|GetLocked?)
    (CallFunction|CheckforKey)
    (else
      (CallFunction|OpenCloseDoor))))

(fn ConstructionScript)

(fn Sounds
  (bind _door (Variables|Default|GetDoor))
  (bind _returnvalue (Transformation|GetWorldLocation _door))
  ;[0 0.06301 0.15] Sounds system
  (if (Variables|Default|GetLocked?)
    (Audio|PlaySoundatLocation (Variables|Default|GetLockedSound) _returnvalue "0, 0, 0" 1.0 1.0 0.0 0 0 0 0)
    (elif (Variables|Default|GetDoorClosed?)
      (Audio|PlaySoundatLocation (Variables|Default|GetOpenSound) _returnvalue "0, 0, 0" 1.0 1.0 0.0 0 0 0 0)
      (else
        (Audio|PlaySoundatLocation (Variables|Default|GetClosedSound) _returnvalue "0, 0, 0" 1.0 1.0 0.0 0 0 0 0)))))