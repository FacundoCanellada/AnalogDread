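; Key pickup actor that, on interaction, adds its KeyID to the BP_FirstPersonFacu player and destroys itself.
; Two sphere triggers drive proximity icons: the outer sphere shows OuterIcon, and the inner sphere swaps it for InnerIcon while the player overlaps.
; The construction script applies icon size, location and both radii from variables, with IconDebug setting icon visibility separately from the runtime HiddenInGame toggles.
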(event OnComponentBeginOverlap(InnerIconCollision)
  (params (OverlappedComponent :type Primitive%20Component%20Object%20Reference) (OtherActor :type Actor%20Object%20Reference) (OtherComp :type Primitive%20Component%20Object%20Reference) (OtherBodyIndex :type Integer) (bFromSweep :type Boolean) (SweepResult :type Hit%20Result%20Structure%20%28by%20ref%29))
  ;[0 0.06301 0.15] Display icons
  (if (== OtherActor (Game|GetPlayerCharacter 0))
    (Development|SetHiddeninGame (Variables|Default|GetInnerIcon) false false)
    (Development|SetHiddeninGame (Variables|Default|GetOuterIcon) true false)))

(event OnComponentEndOverlap(InnerIconCollision)
  (params (OverlappedComponent :type Primitive%20Component%20Object%20Reference) (OtherActor :type Actor%20Object%20Reference) (OtherComp :type Primitive%20Component%20Object%20Reference) (OtherBodyIndex :type Integer))
  ;[0 0.06301 0.15] Display icons
  (if (== (Game|GetPlayerCharacter 0) OtherActor)
    (Development|SetHiddeninGame (Variables|Default|GetInnerIcon) true false)
    (Development|SetHiddeninGame (Variables|Default|GetOuterIcon) false false)))

(event OnComponentBeginOverlap(OuterIconCollision)
  (params (OverlappedComponent :type Primitive%20Component%20Object%20Reference) (OtherActor :type Actor%20Object%20Reference) (OtherComp :type Primitive%20Component%20Object%20Reference) (OtherBodyIndex :type Integer) (bFromSweep :type Boolean) (SweepResult :type Hit%20Result%20Structure%20%28by%20ref%29))
  ;[0 0.06301 0.15] Display icons
  (if (== OtherActor (Game|GetPlayerCharacter 0))
    (Development|SetHiddeninGame (Variables|Default|GetOuterIcon) false false)))

(event OnComponentEndOverlap(OuterIconCollision)
  (params (OverlappedComponent :type Primitive%20Component%20Object%20Reference) (OtherActor :type Actor%20Object%20Reference) (OtherComp :type Primitive%20Component%20Object%20Reference) (OtherBodyIndex :type Integer))
  ;[0 0.06301 0.15] Display icons
  (if (== (Game|GetPlayerCharacter 0) OtherActor)
    (Development|SetHiddeninGame (Variables|Default|GetOuterIcon) true false)))

(event EventBeginPlay
  (bind _asbp_first_person_facu (Utilities|Casting|CastToBP_FirstPersonFacu (Game|GetPlayerCharacter 0)))
  (Variables|Default|SetRefPlayer _asbp_first_person_facu))

(event EventInteraction
  ;[0 0.06301 0.15] Interaction sytem
  (Default|AddKey (Variables|Default|GetRefPlayer) (Variables|Default|GetKey%20ID))
  (Actor|DestroyActor))

(fn ConstructionScript
  (Utilities|FlowControl|Sequence
    (:then_0
      (Transformation|SetWorldScale3D (Variables|Default|GetOuterIcon) (Math|Conversions|ToVector(Float) (Variables|Default|GetIconSize)))
      (Transformation|SetRelativeLocation (Variables|Default|GetOuterIcon) (Variables|Default|GetIconLocation) false false)
      (Rendering|SetVisibility (Variables|Default|GetOuterIcon) (Variables|Default|GetIconDebug) false))
    (:then_1
      (Components|Sphere|SetSphereRadius (Variables|Default|GetInnerIconCollision) (Variables|Default|GetInnerRadius) true)
      (Components|Sphere|SetSphereRadius (Variables|Default|GetOuterIconCollision) (Variables|Default|GetOuterRadius) true))))