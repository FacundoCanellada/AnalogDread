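; BP_InspectItem is an inspectable world item with a configurable mesh, description, voice-over and diary entry.
; InspectItem registers it with the player character, swaps the HUD for a WB_InspectionScreen widget and returns the model.
; A second sequence branch, placed after that return, targets adding the entry to the controller's Diary.
; Separate functions restore the HUD, restart the voice-over and destroy the actor after a short delay; Interaction is empty.
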(event Custom|DestroyItem
  (Utilities|FlowControl|Delay 0.5)
  (Actor|DestroyActor))

(fn ConstructionScript
  (Components|StaticMesh|SetStaticMesh (Variables|Default|GetStaticMesh) (Variables|Default|GetItemModel)))

(fn StopInspectItem
  (bind _returnvalue (Actor|GetActorOfClass "/Game/Facu/Blueprints/Character/BP_FirstPersonFacu.BP_FirstPersonFacu_C"))
  (Widget|SetVisibility (Variables|/Game/Facu/Blueprints/Character/BP_FirstPersonFacu.BP_FirstPersonFacu_C|GetHUDRef _returnvalue) "Visible")
  (Widget|SetVisibility (Variables|Default|GetInspectionScreenRef) "Hidden")
  (Variables|Default|SetInspectionScreenRef 0))

(fn PlayAudio
  (Audio|Components|Audio|Stop (Variables|Default|GetVoiceAudio))
  (Audio|Components|Audio|SetSound (Variables|Default|GetVoiceAudio) (Variables|Default|GetVoiceOverSound))
  (Audio|Components|Audio|Play (Variables|Default|GetVoiceAudio) 0.0))

(fn InspectItem
  (Utilities|FlowControl|Sequence
    (:then_0
      (bind _asbp_first_person_facu (Utilities|Casting|CastToBP_FirstPersonFacu (Game|GetPlayerCharacter 0)))
      (Variables|/Game/Facu/Blueprints/Character/BP_FirstPersonFacu.BP_FirstPersonFacu_C|SetItemReference _asbp_first_person_facu self)
      (bind _returnvalue (Actor|GetActorOfClass "/Game/Facu/Blueprints/Character/BP_FirstPersonFacu.BP_FirstPersonFacu_C"))
      (Widget|SetVisibility (Variables|/Game/Facu/Blueprints/Character/BP_FirstPersonFacu.BP_FirstPersonFacu_C|GetHUDRef _returnvalue) "Hidden")
      (bind _returnvalue_2 (UserInterface|CreateWidget "/Game/Facu/Widgets/WB_InspectionScreen.WB_InspectionScreen_C" 0 (Variables|Default|GetItemDescription)))
      (bind _output_get (Variables|Default|SetInspectionScreenRef _returnvalue_2))
      (UserInterface|Viewport|AddtoViewport _output_get 0)
      (Development|PrintString "Hello")
      (return (Variables|Default|GetItemModel)))
    (:then_1
      (bind _asbp_first_person_player_controller (Utilities|Casting|CastToBP_FirstPersonPlayerController (Game|GetPlayerController 0)))
      (Utilities|IsValid (Variables|/Game/Facu/BP_FirstPersonPlayerController.BP_FirstPersonPlayerController_C|GetDiary _asbp_first_person_player_controller)
        (:Is%20Valid
          (Default|AddEntrytoDiary (Variables|/Game/Facu/BP_FirstPersonPlayerController.BP_FirstPersonPlayerController_C|GetDiary _asbp_first_person_player_controller) (Variables|Default|GetDiaryEntryData))
          (Development|PrintString "Entrada agregada al diario"))))))

(fn Interaction
  (return))