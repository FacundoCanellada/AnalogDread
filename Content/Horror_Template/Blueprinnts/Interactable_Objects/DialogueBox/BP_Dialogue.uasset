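; BP_Dialogue is an interactable dialogue object that shows a speaker's lines one at a time while the game is paused.
; It creates a W_Dialogue widget on BeginPlay.
; Each Speech call pauses the game, sends the current line, speaker name and text delay to the widget, then advances the index.
; The call after the last line resets the index, clears the widget and unpauses the game.
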(event Custom|Speech
  (bind _dialogue (Variables|Default|GetDialogue))
  (Game|SetGamePaused true)
  (Default|IncomingText (Variables|Default|GetDialogueRef) (Utilities|Array|Get(acopy) _dialogue (Variables|Default|GetCurrentDialogue)) (Variables|Default|GetTextDelay) (Variables|Default|GetName))
  (bind _result (Math|Integer|IncrementInt (Variables|Default|GetCurrentDialogue))
    (:%20%20
      (if (>= _result (+ (Utilities|Array|Length _dialogue) 1))
        (Variables|Default|SetCurrentDialogue 0)
        (Default|ClearScreen (Variables|Default|GetDialogueRef))
        (Game|SetGamePaused false)))))

(event EventBeginPlay
  (bind _returnvalue (UserInterface|CreateWidget "/Game/Horror_Template/UI/Widgets/W_Dialogue.W_Dialogue_C"))
  (Variables|Default|SetDialogueRef _returnvalue))