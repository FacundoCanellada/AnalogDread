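; Master Blueprint for a rotating picture frame puzzle, where each frame must reach its answer position.
; Interaction plays a timeline that pitches the picture 90 degrees per step through four positions, and flags it finalized when the next position matches the answer.
; Every frame gathers all frames on BeginPlay and polls them on a looping timer, firing the completion call once all are finalized.
; Tick prints the frame position for debugging.
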(event Custom|RotatePaiting
  (if (not (Variables|Default|GetFrameMoving))
    (Variables|Default|SetFrameMoving true)
    (Audio|PlaySound2D "/Game/Facu/Sounds/SlidePicture.SlidePicture" 1.0 1.0 0.0 0 0)
    (bind _rotation (Timeline|PaitingRotation PlayFromStart)
      (:Update
        (Transformation|SetRelativeRotation (Variables|Default|GetPicture) (Math|Rotator|MakeRotator 0.0 (Math|Float|Lerp (.pitch (Variables|Default|GetStartingRotationFrame)) (- (.pitch (Variables|Default|GetStartingRotationFrame)) 9e+01) _rotation) 0.0) false false))
      (:Finished
        (Variables|Default|SetStartingRotationFrame (Math|Rotator|MakeRotator 0.0 (Math|Float|Lerp (.pitch (Variables|Default|GetStartingRotationFrame)) (- (.pitch (Variables|Default|GetStartingRotationFrame)) 9e+01) _rotation) 0.0))
        (Variables|Default|SetFrameMoving false)
        (bind _result (Math|Integer|IncrementInt (Variables|Default|GetFramePosition))
          (:%20%20
            (bind _output_get (Variables|Default|SetFramePosition _result))
            (if (> _output_get 3)
              (Variables|Default|SetFramePosition 0))))))))

(event Custom|PuzzleCheck
  (Variables|Default|SetPuzzleSolved true)
  (for _array_element (Variables|Default|GetAllPicturesFrame)
    (if (not (Variables|BP_PictureFrameMaster_Puzzle_C|GetFinalized _array_element))
      (Variables|Default|SetPuzzleSolved false)))
  (if (Variables|Default|GetPuzzleSolved)
    (Utilities|Time|ClearandInvalidateTimerbyHandle (stale EventBeginPlay _returnvalue))
    (Default|CallEVDPuzzleCompleted)))

(event EventTick
  (params (DeltaSeconds :type Float%20%28single-precision%29))
  (Development|PrintString (Utilities|String|ToString(Integer) (Variables|Default|GetFramePosition)) true true "(R=0.000000,G=0.660000,B=1.000000,A=1.000000)" DeltaSeconds))

(event EventBeginPlay
  (Variables|Default|SetStartingRotationFrame (Variables|/Script/Engine.SceneComponent|GetRelativeRotation (Variables|Default|GetPicture)))
  (bind _outactors (Actor|GetAllActorsOfClass "BP_PictureFrameMaster_Puzzle_C"))
  (Variables|Default|SetAllPicturesFrame _outactors)
  (bind _returnvalue (Utilities|Time|SetTimerbyEvent (delegate Custom|PuzzleCheck) 0.25 true)))

(event EventInteraction
  (if (== (+ (Variables|Default|GetFramePosition) 1) (Variables|Default|GetPuzzleAnswer))
    (Variables|Default|SetFinalized true)
    (CallFunction|RotatePaiting)
    (else
      (Variables|Default|SetFinalized false)
      (CallFunction|RotatePaiting))))

(fn ConstructionScript
  (|CallParentFunction))