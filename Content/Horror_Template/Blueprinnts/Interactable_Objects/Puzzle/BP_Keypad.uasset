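; Interactable keypad puzzle that unlocks a referenced door when the correct code is entered.
; Interaction blends the view to the keypad, freezes the player and enables mouse clicks; Q exits and restores control.
; Digit buttons feed Code, which plays a sound, updates the widget text and clears input at five digits.
; A match with a valid door reference unlocks it, turns the indicator green and returns control to the player.
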(event OnClicked(button1)
  (params (TouchedComponent :type Primitive%20Component%20Object%20Reference) (ButtonPressed :type Key%20Structure :default "None"))
  (CallFunction|Code "1"))

(event OnClicked(button2)
  (params (TouchedComponent :type Primitive%20Component%20Object%20Reference) (ButtonPressed :type Key%20Structure :default "None"))
  (CallFunction|Code "2"))

(event OnClicked(button3)
  (params (TouchedComponent :type Primitive%20Component%20Object%20Reference) (ButtonPressed :type Key%20Structure :default "None"))
  (CallFunction|Code "3"))

(event OnClicked(button4)
  (params (TouchedComponent :type Primitive%20Component%20Object%20Reference) (ButtonPressed :type Key%20Structure :default "None"))
  (CallFunction|Code "4"))

(event OnClicked(button5)
  (params (TouchedComponent :type Primitive%20Component%20Object%20Reference) (ButtonPressed :type Key%20Structure :default "None"))
  (CallFunction|Code "5"))

(event OnClicked(button6)
  (params (TouchedComponent :type Primitive%20Component%20Object%20Reference) (ButtonPressed :type Key%20Structure :default "None"))
  (CallFunction|Code "6"))

(event OnClicked(button7)
  (params (TouchedComponent :type Primitive%20Component%20Object%20Reference) (ButtonPressed :type Key%20Structure :default "None"))
  (CallFunction|Code "7"))

(event OnClicked(button8)
  (params (TouchedComponent :type Primitive%20Component%20Object%20Reference) (ButtonPressed :type Key%20Structure :default "None"))
  (CallFunction|Code "8"))

(event OnClicked(button9)
  (params (TouchedComponent :type Primitive%20Component%20Object%20Reference) (ButtonPressed :type Key%20Structure :default "None"))
  (CallFunction|Code "9"))

(event OnClicked(button0)
  (params (TouchedComponent :type Primitive%20Component%20Object%20Reference) (ButtonPressed :type Key%20Structure :default "None"))
  (CallFunction|Code "0"))

(event EventInteraction
  (bind _returnvalue (Game|GetPlayerController 0))
  (bind _returnvalue_2 (Game|GetPlayerController 0))
  (Game|Player|SetViewTargetwithBlend _returnvalue_2 self 0.0 "VTBlend_Linear" 0.0 false)
  (Input|SetIgnoreLookInput _returnvalue_2 true)
  (Variables|/Script/Engine.PlayerController|SetbEnableClickEvents _returnvalue_2 true)
  (Variables|/Script/Engine.PlayerController|SetbShowMouseCursor _returnvalue_2 true)
  (Pawn|Components|CharacterMovement|DisableMovement (Variables|/Script/Engine.Character|GetCharacterMovement (Game|GetPlayerCharacter 0)))
  (UserInterface|Viewport|AddtoViewport (Variables|Default|GetKeypadRef) 0)
  (Input|EnableInput _returnvalue)
  (Input|SetInputModeGameandUI _returnvalue 0 "DoNotLock" true false))

(event EventBeginPlay
  (bind _asw_key_pad (Utilities|Casting|CastToW_KeyPad (UserInterface|GetWidget (Variables|Default|GetWidget))))
  (Variables|Default|SetAs%20W%20Key%20Pad _asw_key_pad))

(event Input|KeyboardEvents|Q
  (params (Key :type Key%20Structure :default "None"))
  (:Pressed
    (|Exit)))

(fn ConstructionScript)

(fn Code
  (params (B :type String))
  (bind _returnvalue (Game|GetPlayerCharacter 0))
  (bind _returnvalue_2 (Game|GetPlayerController 0))
  (Audio|PlaySound2D "/Game/Facu/Sounds/KeyPad.KeyPad" 1.0 1.0 0.0 0 0)
  (bind _output_get (Variables|Default|SetInput (Utilities|String|Append (Variables|Default|GetInput) B)))
  (Variables|Default|SetLengthOfCode (+ (Variables|Default|GetLengthOfCode) 1))
  (Rendering|Components|TextRender|SetText (Variables|/Game/Horror_Template/UI/Widgets/W_KeyPad.W_KeyPad_C|GetCodeText (Variables|Default|GetAs%20W%20Key%20Pad)) (Utilities|Text|ToText(String) _output_get))
  (if (Utilities|Enum|Equal(Enum) (Variables|Default|GetInput) (Variables|Default|GetCorrectCode))
    (Utilities|IsValid (Variables|Default|GetDoorReference)
      (:Is%20Valid
        (if true
          (Default|UnlockDoor (Variables|Default|GetDoorReference))
          (Rendering|Material|SetMaterial (Variables|Default|Getspheres) 0 "/Game/Horror_Template/Static_Meshes/Keypad/Materials/MI_KGreen.MI_KGreen")
          (Input|DisableInput _returnvalue_2)
          (Game|Player|SetViewTargetwithBlend _returnvalue_2 _returnvalue 0.3 "VTBlend_Linear" 0.0 false)
          (Input|ResetIgnoreLookInput _returnvalue_2)
          (Variables|/Script/Engine.PlayerController|SetbEnableClickEvents _returnvalue_2 false)
          (Variables|/Script/Engine.PlayerController|SetbShowMouseCursor _returnvalue_2 false)
          (Pawn|Components|CharacterMovement|SetMovementMode (Variables|/Script/Engine.Character|GetCharacterMovement _returnvalue) "MOVE_Walking" 0)
          (Input|SetInputModeGameOnly _returnvalue_2 false)
          (if (>= (Variables|Default|GetLengthOfCode) 5) :!label _label
            (bind _output_get_2 (Variables|Default|SetInput ""))
            (Rendering|Components|TextRender|SetText (Variables|/Game/Horror_Template/UI/Widgets/W_KeyPad.W_KeyPad_C|GetCodeText (Variables|Default|GetAs%20W%20Key%20Pad)) (Utilities|Text|ToText(String) _output_get_2))
            (Variables|Default|SetLengthOfCode 0)))))
    (else
      (goto _label))))